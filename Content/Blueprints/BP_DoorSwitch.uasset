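; BP_DoorSwitch is an interactable switch that opens a linked door when the player presses E nearby.
; Sphere overlap events set an in-range flag while BP_FirstPersonCharacter is inside, filtering other actors by cast.
; The E key event checks that flag and calls OpenDoor on the DoorToOpen reference.
; A leftover custom event branches on IsDoorOpen but performs no action.
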(event `CustomEvent`
  (if (not (`self.IsDoorOpen`))
    _))

(event `Key|E` :consume false
  (params (Key :type "Key Structure"))
  (:`Pressed`
    (if (`self.PLayerInRange`)
      (`/Game/Blueprints/BP_Door.OpenDoor` (`self.DoorToOpen`)))))

(event `self.Sphere.OnComponentBeginOverlap`
  (params (OverlappedComponent :type "PrimitiveComponent Object Reference") (OtherActor :type "Actor Object Reference") (OtherComp :type "PrimitiveComponent Object Reference") (OtherBodyIndex :type Integer) (bFromSweep :type Boolean) (SweepResult :type "HitResult Structure (by ref)"))
  (cast `/Game/FirstPerson/Blueprints/BP_FirstPersonCharacter` OtherActor)
  (set `self.PLayerInRange` true))

(event `self.Sphere.OnComponentEndOverlap`
  (params (OverlappedComponent :type "PrimitiveComponent Object Reference") (OtherActor :type "Actor Object Reference") (OtherComp :type "PrimitiveComponent Object Reference") (OtherBodyIndex :type Integer))
  (cast `/Game/FirstPerson/Blueprints/BP_FirstPersonCharacter` OtherActor)
  (set `self.PLayerInRange` false))

(fn `UserConstructionScript`)