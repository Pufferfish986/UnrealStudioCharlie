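; Blueprint that procedurally assembles a small, simple house out of basic meshes when play begins.
; BeginPlay adds six static mesh components at runtime, each placed with hard-coded relative transforms.
; Scaled cubes form the foundation and three walls, and two opposite-facing ramps form the roof.
; The construction script is empty, so none of this geometry is built in the editor viewport.
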(event `self.ReceiveBeginPlay`
  ; foundation
  (bind _returnvalue (`AddComponent|NODE_AddStaticMeshComponent-0`))
  (`StaticMeshComponent.SetStaticMesh` _returnvalue "/Game/LevelPrototyping/Meshes/SM_Cube.SM_Cube")
  (`SceneComponent.K2_SetRelativeLocation` _returnvalue (0.0 0.0 0.0) false false)
  (`SceneComponent.K2_SetRelativeLocation` _returnvalue (0.0 0.0 0.0) false false)
  (`SceneComponent.SetRelativeScale3D` _returnvalue (1.0 1.0 0.1))
  (bind _returnvalue_2 (`AddComponent|NODE_AddStaticMeshComponent-1`))
  (`StaticMeshComponent.SetStaticMesh` _returnvalue_2 "/Game/LevelPrototyping/Meshes/SM_Cube.SM_Cube")
  (`SceneComponent.K2_SetRelativeLocation` _returnvalue_2 (0.0 0.0 0.0) false false)
  (`SceneComponent.SetRelativeScale3D` _returnvalue_2 (1.0 0.1 1.0))
  ; wall3
  (bind _returnvalue_3 (`AddComponent|NODE_AddStaticMeshComponent-2`))
  (`StaticMeshComponent.SetStaticMesh` _returnvalue_3 "/Game/LevelPrototyping/Meshes/SM_Cube.SM_Cube")
  (`SceneComponent.K2_SetRelativeLocation` _returnvalue_3 (100.0 0.0 0.0) false false)
  (`SceneComponent.SetRelativeScale3D` _returnvalue_3 (1.0 0.1 1.0))
  (`SceneComponent.K2_SetRelativeRotation` _returnvalue_3 (struct :`Yaw` 90.0) false false)
  ; 注释
  (bind _returnvalue_4 (`AddComponent|NODE_AddStaticMeshComponent-3`))
  (`StaticMeshComponent.SetStaticMesh` _returnvalue_4 "/Game/LevelPrototyping/Meshes/SM_Cube.SM_Cube")
  (`SceneComponent.K2_SetRelativeLocation` _returnvalue_4 (0.0 90.0 0.0) false false)
  (`SceneComponent.SetRelativeScale3D` _returnvalue_4 (1.0 0.1 1.0))
  (`SceneComponent.K2_SetRelativeRotation` _returnvalue_4 (struct) false false)
  ; 注释
  (bind _returnvalue_5 (`AddComponent|NODE_AddStaticMeshComponent-4`))
  (`StaticMeshComponent.SetStaticMesh` _returnvalue_5 "/Game/LevelPrototyping/Meshes/SM_Ramp.SM_Ramp")
  (`SceneComponent.K2_SetRelativeLocation` _returnvalue_5 (100.0 50.0 100.0) false false)
  (`SceneComponent.SetRelativeScale3D` _returnvalue_5 (1.0 0.6 0.5))
  (`SceneComponent.K2_SetRelativeRotation` _returnvalue_5 (struct :`Yaw` 180.0) false false)
  ; 注释
  (bind _returnvalue_6 (`AddComponent|NODE_AddStaticMeshComponent-5`))
  (`StaticMeshComponent.SetStaticMesh` _returnvalue_6 "/Game/LevelPrototyping/Meshes/SM_Ramp.SM_Ramp")
  (`SceneComponent.K2_SetRelativeLocation` _returnvalue_6 (0.0 50.0 100.0) false false)
  (`SceneComponent.SetRelativeScale3D` _returnvalue_6 (1.0 0.6 0.5))
  (`SceneComponent.K2_SetRelativeRotation` _returnvalue_6 (struct) false false))

(fn `MyVariable`)

(fn `UserConstructionScript`)