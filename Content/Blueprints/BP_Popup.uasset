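; BP_Popup is a trigger actor that toggles a WBP_PopupParent UI popup when something begins overlapping its box.
; Each overlap flips a visibility flag, either creating the widget and adding it to the viewport or removing it.
; Showing the popup switches to game-and-UI input with a visible mouse cursor; hiding it restores game-only input.
; The overlap does not filter which actor entered, and leaving the box does nothing.
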(event `self.Box.OnComponentBeginOverlap`
  (params (OverlappedComponent :type "PrimitiveComponent Object Reference") (OtherActor :type "Actor Object Reference") (OtherComp :type "PrimitiveComponent Object Reference") (OtherBodyIndex :type Integer) (bFromSweep :type Boolean) (SweepResult :type "HitResult Structure (by ref)"))
  (bind _returnvalue (`GameplayStatics.GetPlayerController` 0))
  (if (`self.IsVisible`)
    (`Widget.RemoveFromParent` (stale _returnvalue_2))
    (set `self.IsVisible` false)
    (`WidgetBlueprintLibrary.SetInputMode_GameOnly` _returnvalue)
    (set `PlayerController.bShowMouseCursor` false _returnvalue)
    (else
      (bind _returnvalue_2 (`|CreateWidget` "/Game/Blueprints/WBP_PopupParent.WBP_PopupParent_C"))
      (`UserWidget.AddToViewport` _returnvalue_2 0)
      (set `self.IsVisible` true)
      (`WidgetBlueprintLibrary.SetInputMode_GameAndUIEx` _returnvalue null)
      (set `PlayerController.bShowMouseCursor` true _returnvalue)
      (if (`self.IsVisible`)
        _))))

(fn `UserConstructionScript`)